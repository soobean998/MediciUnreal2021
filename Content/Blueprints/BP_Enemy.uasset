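; BP_Enemy is an enemy actor that travels in a straight line at a fixed speed.
; On BeginPlay it casts the player pawn to BP_Player, then randomly picks its direction using DirRate as a percent chance: straight down the Z axis, otherwise toward the player's position at that moment.
; Tick moves it along that unchanging direction without sweeping, and the overlap event is empty.
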(event EventBeginPlay
  (bind _asbp_player (Utilities|Casting|CastToBP_Player (Game|Player|GetPlayerPawn 0)))
  (if (< (Math|Random|RandomIntegerinRange 0 99) (Variables|Default|GetDirRate))
    (Variables|Default|SetMoveDirection "0,0.000000,-1.000000")
    (else
      (Variables|Default|SetMoveDirection (Math|Vector|Normalize (- (Transformation|GetActorLocation _asbp_player) (Transformation|GetActorLocation)))))))

(event Collision|EventActorBeginOverlap
  (params (OtherActor :type Actor%20Object%20Reference)))

(event EventTick
  (params (DeltaSeconds :type Float%20%28single-precision%29))
  (Transformation|SetActorLocation (+ (Transformation|GetActorLocation) (* (* (Variables|Default|GetMoveDirection) (Variables|Default|GetMoveSpeed)) DeltaSeconds)) false false))

(fn ConstructionScript)