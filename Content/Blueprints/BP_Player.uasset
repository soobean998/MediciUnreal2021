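; BP_Player is the player-controlled actor of a shooter, moving on the Y-Z plane and firing bullets.
; Each Tick it normalizes the Horizontal and Vertical input, scales it by MoveSpeed and DeltaSeconds, and offsets its location without sweeping.
; Pressing Fire1 calls FireBullet, which spawns BP_Bullet at the SpawnArrow location, prints a Korean missile-fired message and plays a blaster sound at the world origin.
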(event EventBeginPlay)

(event Collision|EventActorBeginOverlap
  (params (OtherActor :type Actor%20Object%20Reference)))

(event EventTick
  (params (DeltaSeconds :type Float%20%28single-precision%29))
  ;[1 1 1] 플레이어 이동 공식(p = p0 +vt)
  (Transformation|SetActorLocation (+ (Transformation|GetActorLocation) (* (* (Math|Vector|Normalize (Math|Vector|MakeVector 0.0 (Input|AxisValues|GetHorizontal) (Input|AxisValues|GetVertical))) (Variables|PlayerSettings|GetMoveSpeed)) DeltaSeconds)) false false))

(event Input|ActionEvents|InputActionFire1
  (params (Key :type Key%20Structure))
  (:Pressed
    (CallFunction|FireBullet)))

(fn ConstructionScript)

(fn FireBullet
  (Game|SpawnActorfromClass "/Game/Blueprints/BP_Bullet.BP_Bullet_C" (Math|Transform|MakeTransform (Transformation|GetWorldLocation (Variables|Default|GetSpawnArrow)) "0, 0, 0" "1,1,1") "AlwaysSpawn" 0 0)
  (Development|PrintString "미사일이 발사됐어요!")
  (Audio|PlaySoundatLocation "/Game/Sounds/star-wars-blaster.star-wars-blaster" "0, 0, 0" "0, 0, 0" 1.0 1.0 0.0 0 0 0))